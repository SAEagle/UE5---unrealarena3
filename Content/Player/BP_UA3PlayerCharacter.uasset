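; UA3 player character Blueprint that layers spawn audio, death weapon drops and weapon UI timing onto the character.
; Tick polls HealthComponent and, on death, hides the widget and once spawns a one-time shotgun, launcher or plasma pickup matching the current weapon.
; Tick also clears the UI helper's pickup-added flag after a delay, a debug stopgap awaiting C++.
; Weapon key presses clear CanHideTab, which is restored five seconds after release.
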(event `self.ReceiveBeginPlay`
  (`GameplayStatics.PlaySound2D` "/Game/Sounds/Character/SCue_CharacterSpawn.SCue_CharacterSpawn" 1.0 1.0 0.0 null null))

(event `self.ReceiveTick`
  (params (DeltaSeconds :type "Float (single-precision)"))
  (bind _returnvalue (`self.K2_GetActorLocation`))
  (bind _uihelpercomponent (`self.UIHelperComponent`))
  (bind _weaponcomponent (`self.WeaponComponent`))
  (`|ExecutionSequence`
    (:`then_0`
      (if (`UA3HealthComponent.IsDead` (`self.HealthComponent`))
        (`SceneComponent.SetVisibility` (`self.Widget`) true false)
        (`/Engine/EditorBlueprintResources/StandardMacros.DoOnce` false
          (:`Completed`
            (`self.SpawnWeapon`)
            (if (`UA3WeaponComponent.GetCurrentWeaponIndex` _weaponcomponent 2)
              (bind _returnvalue_2 (`|SpawnActorFromClass` "/Game/Pickups/BP_UA3ShotgunPickup.BP_UA3ShotgunPickup_C" (`KismetMathLibrary.MakeTransform` _returnvalue) "Undefined" "OverrideRootScale" null null))
              (set `UA3BasePickup.OneTimeSpawner` true _returnvalue_2)
              (elif (`UA3WeaponComponent.GetCurrentWeaponIndex` _weaponcomponent 3)
                (bind _returnvalue_3 (`|SpawnActorFromClass` "/Game/Pickups/BP_UA3LauncherPickup.BP_UA3LauncherPickup_C" (`KismetMathLibrary.MakeTransform` _returnvalue) "Undefined" "OverrideRootScale" null null))
                (set `UA3BasePickup.OneTimeSpawner` true _returnvalue_3)
                (elif (`UA3WeaponComponent.GetCurrentWeaponIndex` _weaponcomponent 4)
                  (bind _returnvalue_4 (`|SpawnActorFromClass` "/Game/Pickups/BP_UA3PlasmaPickup.BP_UA3PlasmaPickup_C" (`KismetMathLibrary.MakeTransform` _returnvalue) "Undefined" "OverrideRootScale" null null))
                  (set `UA3BasePickup.OneTimeSpawner` true _returnvalue_4))))))))
    (:`then_1`
      ;[1 1 1] Debug Need to add later in C++
      (if (`UA3UIHelperComponent.GetPickupAdded` _uihelpercomponent)
        (`KismetSystemLibrary.Delay` 1.0)
        (`UA3UIHelperComponent.SetPickupAdded` _uihelpercomponent false)))))

(event `Key|Q`
  (params (Key :type "Key Structure"))
  ;[1 1 1] Weapon Events
  (:`Pressed`
    (set `self.CanHideTab?` false))
  (:`Released`
    (`KismetSystemLibrary.Delay` 5.0)
    (set `self.CanHideTab?` true)))

(event `Key|One`
  (params (Key :type "Key Structure"))
  ;[1 1 1] Weapon Events
  (:`Pressed`
    (set `self.CanHideTab?` false))
  (:`Released`
    (`KismetSystemLibrary.Delay` 5.0)
    (set `self.CanHideTab?` true)))

(event `Key|Two`
  (params (Key :type "Key Structure"))
  ;[1 1 1] Weapon Events
  (:`Pressed`
    (set `self.CanHideTab?` false))
  (:`Released`
    (`KismetSystemLibrary.Delay` 5.0)
    (set `self.CanHideTab?` true)))

(event `Key|Three`
  (params (Key :type "Key Structure"))
  ;[1 1 1] Weapon Events
  (:`Pressed`
    (set `self.CanHideTab?` false))
  (:`Released`
    (`KismetSystemLibrary.Delay` 5.0)
    (set `self.CanHideTab?` true)))

(event `Key|Five`
  (params (Key :type "Key Structure"))
  ;[1 1 1] Weapon Events
  (:`Pressed`
    (set `self.CanHideTab?` false))
  (:`Released`
    (`KismetSystemLibrary.Delay` 5.0)
    (set `self.CanHideTab?` true)))

(event `Key|Eight`
  (params (Key :type "Key Structure"))
  ;[1 1 1] Weapon Events
  (:`Pressed`
    (set `self.CanHideTab?` false))
  (:`Released`
    (`KismetSystemLibrary.Delay` 5.0)
    (set `self.CanHideTab?` true)))

(fn `UserConstructionScript`)