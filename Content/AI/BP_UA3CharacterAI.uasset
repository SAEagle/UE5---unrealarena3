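; BP_UA3CharacterAI is an AI-controlled character that drops a weapon pickup when it dies.
; It plays a 2D spawn sound on BeginPlay, then polls its HealthComponent every Tick for death.
; While dead it shows its Widget, and a DoOnce calls SpawnWeapon and checks the WeaponComponent's current weapon index.
; A matching shotgun, launcher or plasma pickup spawns at the actor's location, flagged as a one-time spawner.
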(event `self.ReceiveBeginPlay`
  (`GameplayStatics.PlaySound2D` "/Game/Sounds/Character/SCue_CharacterSpawn.SCue_CharacterSpawn" 1.0 1.0 0.0 null null))

(event `self.ReceiveTick`
  (params (DeltaSeconds :type "Float (single-precision)"))
  (bind _returnvalue (`self.K2_GetActorLocation`))
  (bind _weaponcomponent (`self.WeaponComponent`))
  (if (`UA3HealthComponent.IsDead` (`self.HealthComponent`))
    (`SceneComponent.SetVisibility` (`self.Widget`) true false)
    (`/Engine/EditorBlueprintResources/StandardMacros.DoOnce` false
      (:`Completed`
        (`self.SpawnWeapon`)
        (if (`UA3WeaponComponent.GetCurrentWeaponIndex` _weaponcomponent 1)
          (bind _returnvalue_2 (`|SpawnActorFromClass` "/Game/Pickups/BP_UA3ShotgunPickup.BP_UA3ShotgunPickup_C" (`KismetMathLibrary.MakeTransform` _returnvalue) "Undefined" "OverrideRootScale" null null))
          (set `UA3BasePickup.OneTimeSpawner` true _returnvalue_2)
          (elif (`UA3WeaponComponent.GetCurrentWeaponIndex` _weaponcomponent 2)
            (bind _returnvalue_3 (`|SpawnActorFromClass` "/Game/Pickups/BP_UA3LauncherPickup.BP_UA3LauncherPickup_C" (`KismetMathLibrary.MakeTransform` _returnvalue) "Undefined" "OverrideRootScale" null null))
            (set `UA3BasePickup.OneTimeSpawner` true _returnvalue_3)
            (elif (`UA3WeaponComponent.GetCurrentWeaponIndex` _weaponcomponent 3)
              (bind _returnvalue_4 (`|SpawnActorFromClass` "/Game/Pickups/BP_UA3PlasmaPickup.BP_UA3PlasmaPickup_C" (`KismetMathLibrary.MakeTransform` _returnvalue) "Undefined" "OverrideRootScale" null null))
              (set `UA3BasePickup.OneTimeSpawner` true _returnvalue_4))))))))

(fn `UserConstructionScript`)